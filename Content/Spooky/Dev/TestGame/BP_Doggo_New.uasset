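; BP_Doggo_New is a dog actor that glides to a randomly chosen position, relative to where it spawned.
; SelectNextPosition picks an offset from Positions, records start time and location, and disables interaction; BeginPlay makes the first call.
; Tick linearly interpolates the root over Duration, then holds it at the target and sets CanInteract.
; Nothing in this Blueprint triggers moves after the first.
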(event EventBeginPlay
  (Variables|Default|SetInitialWorldPosition (Transformation|GetWorldLocation (Variables|Default|GetDefaultSceneRoot)))
  (Utilities|SelectNextPosition))

(event EventTick
  (params (DeltaSeconds :type Float%20%28single-precision%29))
  (bind _returnvalue (Utilities|Time|GetGameTimeinSeconds))
  (bind _defaultsceneroot (Variables|Default|GetDefaultSceneRoot))
  (bind _initialworldposition (Variables|Default|GetInitialWorldPosition))
  (bind _targetposition (Variables|Default|GetTargetPosition))
  (bind _starttime (Variables|Default|GetStartTime))
  (bind _duration (Variables|Default|GetDuration))
  (bind _returnvalue_2 (- _returnvalue _starttime))
  (bind _returnvalue_3 (+ _initialworldposition _targetposition))
  (if (>= _duration _returnvalue_2)
    (Transformation|SetWorldLocation _defaultsceneroot (Math|Vector|Lerp(Vector) (Variables|Default|GetStartPosition) _returnvalue_3 (/ _returnvalue_2 _duration)) false false)
    (else
      (Transformation|SetWorldLocation _defaultsceneroot _returnvalue_3 false false)
      (Variables|Default|SetCanInteract true))))

(fn ConstructionScript)