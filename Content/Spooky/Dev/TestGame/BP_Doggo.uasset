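; BP_Doggo is a catchable dog that moves along preset points when caught, in a test game.
; Overlap with BP_Personnage on the CatchTheDoggo component shows a prompt widget and toggles IsCatchable.
; The construction script turns Positions into relative Movement control points, adding one second of duration each.
; CatchedDoggo, when catchable, prints a message and runs Movement for one second, roughly one segment per catch.
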(event OnComponentBeginOverlap(CatchTheDoggo)
  (params (OverlappedComponent :type Primitive%20Component%20Object%20Reference) (OtherActor :type Actor%20Object%20Reference) (OtherComp :type Primitive%20Component%20Object%20Reference) (OtherBodyIndex :type Integer) (bFromSweep :type Boolean) (SweepResult :type Hit%20Result%20Structure%20%28by%20ref%29))
  (Utilities|Casting|CastToBP_Personnage OtherActor)
  (bind _returnvalue (UserInterface|CreateWidget "/Game/Spooky/Dev/TestGame/CatchTheDoggoWidget.CatchTheDoggoWidget_C"))
  (UserInterface|Viewport|AddtoViewport _returnvalue 0)
  (Variables|Default|SetIsCatchable true))

(event OnComponentEndOverlap(CatchTheDoggo)
  (params (OverlappedComponent :type Primitive%20Component%20Object%20Reference) (OtherActor :type Actor%20Object%20Reference) (OtherComp :type Primitive%20Component%20Object%20Reference) (OtherBodyIndex :type Integer))
  (Utilities|Casting|CastToBP_Personnage OtherActor)
  (Widget|RemovefromParent (stale OnComponentBeginOverlap(CatchTheDoggo) _returnvalue))
  (Variables|Default|SetIsCatchable false))

(event Custom|CatchedDoggo
  (bind _movement (Variables|Default|GetMovement))
  (if (Variables|Default|GetIsCatchable)
    ;[1 1 1] TODO Changement position
    (Development|PrintString "You catched the doggo" true true "(R=0.000000,G=0.660000,B=1.000000,A=1.000000)" 2.0 "Catched")
    (Components|Activation|Activate _movement false)
    (Utilities|FlowControl|Delay 1.0)
    (Components|Activation|Deactivate _movement)))

(fn ConstructionScript
  (bind _movement (Variables|Default|GetMovement))
  (Components|Activation|SetAutoActivate (Variables|Default|GetMovement) false)
  (Class|InterptoMovementComponent|AddControlPointPosition (Variables|Default|GetMovement) "0, 0, 0" true)
  (for _array_element (Variables|Default|GetPositions)
    (bind _output_get (Variables|/Script/Engine.InterpToMovementComponent|SetDuration _movement (+ (stale _output_get) 1.0)))
    (Class|InterptoMovementComponent|AddControlPointPosition _movement _array_element true)))